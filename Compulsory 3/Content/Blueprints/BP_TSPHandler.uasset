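; Handler actor for a Travelling Salesman Problem demo, linking its on-screen widget to node spawning and the nearest-neighbour solver.
; On BeginPlay it creates the TSP widget and binds its buttons to resetting the spawner, spawning initial nodes and running HandleNearestNeighbour.
; FoundTotalDistanceEvent writes the total distance to the widget's text block.
; The spawning and solving logic lives outside these graphs.
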(event `NearsetNeighbour`
  (`self.HandleNearestNeighbour`))

(event `ResetEvent`
  (`NodeSpawner.ResetSpawner` (`self.nodeSpawner`)))

(event `Spawn`
  (`NodeSpawner.SpawnInitialNodes` (`self.nodeSpawner`)))

(event `self.ReceiveBeginPlay`
  (bind _returnvalue (`|CreateWidget` "/Game/UI/TSPWidget.TSPWidget_C"))
  (`UserWidget.AddToViewport` _returnvalue 0)
  (set `self.TSPWidget` _returnvalue)
  (add `/Game/UI/BasicButton.Clicked` (`/Game/UI/TSPWidget.ResetSpawner` (`self.TSPWidget`)) (delegate `ResetEvent`))
  (add `/Game/UI/BasicButton.Clicked` (`/Game/UI/TSPWidget.SpawnNodes` (`self.TSPWidget`)) (delegate `Spawn`))
  (add `/Game/UI/BasicButton.Clicked` (`/Game/UI/TSPWidget.NearestNeighbour` (`self.TSPWidget`)) (delegate `NearsetNeighbour`)))

(event `self.FoundTotalDistanceEvent`
  (params (distance :type "Float (single-precision)"))
  (`TextBlock.SetText` (`/Game/UI/TSPWidget.DistanceTEXTBLOCK` (`self.TSPWidget`)) (`KismetTextLibrary.Conv_DoubleToText` distance "HalfToEven")))

(fn `UserConstructionScript`)