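; Level handler for a Travelling Salesman Problem demo that links the TSP UI to node spawning and solving.
; On BeginPlay it creates the TSP widget and binds its buttons to reset the node spawner, spawn initial nodes, or run the nearest-neighbour heuristic.
; An event receiving the computed total distance writes it to the widget's distance text.
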(event `RunNearestNeighbourEvent`
  (`self.HandleNearestNeighbour`))

(event `ResetSpawnerEvent`
  (`NodeSpawner.ResetSpawner` (`self.nodeSpawner`)))

(event `SpawnNodesEvent`
  (`NodeSpawner.SpawnInitialNodes` (`self.nodeSpawner`)))

(event `self.FoundTotalDistanceEvent`
  (params (distance :type "Float (single-precision)"))
  (`TextBlock.SetText` (`/Game/UI/TSPWidget.DistanceTEXTBLOCK` (`self.TSPWidget`)) (`KismetTextLibrary.Conv_DoubleToText` distance "HalfToEven")))

(event `self.ReceiveBeginPlay`
  (bind _returnvalue (`|CreateWidget` "/Game/UI/TSPWidget.TSPWidget_C"))
  (`UserWidget.AddToViewport` _returnvalue 0)
  (set `self.TSPWidget` _returnvalue)
  (add `/Game/UI/BasicButton.Clicked` (`/Game/UI/TSPWidget.ResetSpawner` (`self.TSPWidget`)) (delegate `ResetSpawnerEvent`))
  (add `/Game/UI/BasicButton.Clicked` (`/Game/UI/TSPWidget.SpawnNodes` (`self.TSPWidget`)) (delegate `SpawnNodesEvent`))
  (add `/Game/UI/BasicButton.Clicked` (`/Game/UI/TSPWidget.NearestNeighbour` (`self.TSPWidget`)) (delegate `RunNearestNeighbourEvent`)))

(fn `UserConstructionScript`)